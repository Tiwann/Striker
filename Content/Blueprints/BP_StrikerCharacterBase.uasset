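; Base striker character that the player moves in world-space directions with Enhanced Input.
; BeginPlay adds the player mapping context, and the Move action stores or clears a direction vector.
; While a direction is held, Tick overwrites the capsule's physics linear velocity at MoveSpeed, rather than using movement input, and smoothly turns the actor's yaw toward that direction.
; Releasing input stops these updates without zeroing the velocity.
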(event `self.ReceiveBeginPlay`
  (bind _asplayer_controller (cast `PlayerController` (`self.GetController`)))
  (bind _returnvalue (pcsubsystem `EnhancedInputLocalPlayerSubsystem` _asplayer_controller))
  (`/Engine/EditorBlueprintResources/StandardMacros.IsValid` _returnvalue
    (:`Is Valid`
      (message `EnhancedInputSubsystemInterface.AddMappingContext` _returnvalue "/Game/Input/IMC_Player.IMC_Player" 0 (struct)))))

(event `EnhancedInput|/Game/Input/IPA_Move`
  (params (ActionValue :type "Vector2D Structure") (ElapsedSeconds :type "Float (double-precision)") (TriggeredSeconds :type "Float (double-precision)") (InputAction :type "InputAction Object Reference" :default "/Game/Input/IPA_Move.IPA_Move"))
  (:`Triggered`
    (set `self.MoveDirection` (`KismetMathLibrary.Conv_Vector2DToVector` ActionValue)))
  (:`Completed`
    (set `self.MoveDirection` (0.0 0.0 0.0))))

(event `self.ReceiveTick`
  (params (DeltaSeconds :type "Float (single-precision)"))
  (if (not (`KismetMathLibrary.Vector_IsZero` (`self.MoveDirection`)))
    (`PrimitiveComponent.SetPhysicsLinearVelocity` (`self.Capsule`) (`self.Get Mouvement Vector` (`self.MoveDirection`) (`self.MoveSpeed`)) false "None")
    (`self.K2_SetActorRotation` (`KismetMathLibrary.RInterpTo` (`self.K2_GetActorRotation`) (`KismetMathLibrary.MakeRotator` 0.0 0.0 (`KismetMathLibrary.ClampAxis` (`self.GetRotationAngleFromDirection` (`self.MoveDirection`)))) (`GameplayStatics.GetWorldDeltaSeconds`) 10.0))))

(fn `Get Mouvement Vector`
  (params (MoveDirection :type "Vector Structure") (Speed :type "Float (double-precision)"))
  (returns (ReturnValue :type "Vector Structure"))
  (return (* (`KismetMathLibrary.Normal` (`KismetMathLibrary.MakeVector` MoveDirection_Y MoveDirection_X MoveDirection_Z)) Speed)))

(fn `GetRotationAngleFromDirection`
  (params (Direction :type "Vector Structure"))
  (returns (ReturnValue :type "Float (double-precision)"))
  (return (`KismetMathLibrary.DegAtan2` Direction_X Direction_Y)))

(fn `UserConstructionScript`)